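; BP_Projectile is a launchable ball projectile that also carries its own spawn helpers; its event graph is empty.
; Launch applies a forward velocity-change impulse to the static mesh, and PrintYourName prints the actor's display name.
; SpawnBall spawns a new projectile, but its branch is hardwired true, so Ammo and CheckAmmoPositive go unused.
; AddImpulseToBall is empty, and the player-based spawn transform is left unconnected.
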(fn `AddImpulseToBall`)

(fn `CheckAmmoPositive`
  (params (ammo :type Integer))
  (returns (ammo_positive :type Boolean))
  (return (> ammo 0)))

(fn `Launch`
  (bind _staticmeshcomponent (`self.StaticMeshComponent`))
  (`PrimitiveComponent.AddImpulse` _staticmeshcomponent (* (`SceneComponent.GetForwardVector` _staticmeshcomponent) 1000.0) "None" true))

(fn `PrintYourName`
  (`KismetSystemLibrary.PrintString` (`KismetSystemLibrary.GetDisplayName` self)))

(fn `SpawnBall`
  (params (ammo :type Integer))
  (returns (ReturnValue :type "/Game/BP_Projectile Object Reference"))
  (bind _returnvalue (`GameplayStatics.GetPlayerPawn` 0))
  (if true
    (bind _returnvalue_2 (`|SpawnActorFromClass` "BP_Projectile_C" (`KismetMathLibrary.MakeTransform` (`self.K2_GetActorLocation` _returnvalue) (`Pawn.GetControlRotation` _returnvalue)) "Undefined" "OverrideRootScale" null null))
    (else
      (`KismetSystemLibrary.PrintString` "out of ammo")))
  (return _returnvalue_2))

(fn `UserConstructionScript`)